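; Draft interactable NPC that offers a named "Talk to" prompt and opens a data-table-driven dialogue.
; Interaction overlap events register the NPC with the player's BP_PlayerInteractionComponent and toggle the prompt, while Tick also polls overlap but registers the player instead.
; Interact enters dialogue mode and shows WBP_DialogueBox from the "Start" line.
; Its close event, also triggerable through ForceEndDialogue, removes the box, exits dialogue mode and restores the prompt.
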(event `self.ReceiveBeginPlay`)

(event `self.ReceiveTick`
  (params (DeltaSeconds :type "Float (single-precision)"))
  (bind _returnvalue (`GameplayStatics.GetPlayerCharacter` 0))
  (bind _interactionwidget (`self.InteractionWidget`))
  (if (`PrimitiveComponent.IsOverlappingActor` (`self.Interaction`) _returnvalue)
    (bind _ascharacter (cast `Character` _returnvalue))
    (bind _output_get (set `self.OverlappingPlayer` _ascharacter))
    (`/Game/Blueprints/Systems/BP_PlayerInteractionComponent.SetCurrentInteractable` (`self.GetComponentByClass` _ascharacter "/Game/Blueprints/Systems/BP_PlayerInteractionComponent.BP_PlayerInteractionComponent_C") _output_get)
    (bind _aswbp_interaction_prompt (cast `/Game/UI/WBP_InteractionPrompt` (`WidgetComponent.GetUserWidgetObject` _interactionwidget) :!label _label))
    (bind _prompttext (`/Game/Blueprints/Systems/BPI_Interactable.GetInteractionPrompt`))
    (`TextBlock.SetText` (`/Game/UI/WBP_InteractionPrompt.PromptTextBlock` _aswbp_interaction_prompt) _prompttext)
    (`SceneComponent.SetVisibility` _interactionwidget true false)))

(event `self.Interaction.OnComponentBeginOverlap`
  (params (OverlappedComponent :type "PrimitiveComponent Object Reference") (OtherActor :type "Actor Object Reference") (OtherComp :type "PrimitiveComponent Object Reference") (OtherBodyIndex :type Integer) (bFromSweep :type Boolean) (SweepResult :type "HitResult Structure (by ref)"))
  (bind _ascharacter (cast `Character` OtherActor))
  (`KismetSystemLibrary.PrintString` "Player in range")
  (set `self.OverlappingPlayer` _ascharacter)
  (`/Game/Blueprints/Systems/BP_PlayerInteractionComponent.SetCurrentInteractable` (`self.GetComponentByClass` _ascharacter "/Game/Blueprints/Systems/BP_PlayerInteractionComponent.BP_PlayerInteractionComponent_C") self)
  (goto _label))

(event `self.Interaction.OnComponentEndOverlap`
  (params (OverlappedComponent :type "PrimitiveComponent Object Reference") (OtherActor :type "Actor Object Reference") (OtherComp :type "PrimitiveComponent Object Reference") (OtherBodyIndex :type Integer))
  (bind _ascharacter (cast `Character` OtherActor))
  (`KismetSystemLibrary.PrintString` "Player left range")
  (set `self.OverlappingPlayer` null)
  (`/Game/Blueprints/Systems/BP_PlayerInteractionComponent.SetCurrentInteractable` (`self.GetComponentByClass` _ascharacter "/Game/Blueprints/Systems/BP_PlayerInteractionComponent.BP_PlayerInteractionComponent_C") null)
  (`SceneComponent.SetVisibility` (`self.InteractionWidget`) false false))

(event `/Game/Blueprints/Systems/BPI_Interactable.Interact`
  (params (Instigator :type "Actor Object Reference"))
  (`KismetSystemLibrary.PrintString` "Interact called on NPC")
  (`/Game/Blueprints/Systems/BPI_Interactable.SetInteractionPromptVisible` false)
  (`/Game/Blueprints/Systems/BP_PlayerInteractionComponent.EnterDialogueMode` (`self.GetComponentByClass` Instigator "/Game/Blueprints/Systems/BP_PlayerInteractionComponent.BP_PlayerInteractionComponent_C"))
  (bind _returnvalue (`|CreateWidget` "/Game/UI/WBP_DialogueBox.WBP_DialogueBox_C"))
  (`UserWidget.SetAnchorsInViewport` _returnvalue (make `Anchors` (0.5 0.75) (0.5 0.75)))
  (`UserWidget.SetAlignmentInViewport` _returnvalue (0.5 0.75))
  (bind _output_get (set `self.ActiveDialogueWidget` _returnvalue))
  (set `/Game/UI/WBP_DialogueBox.DialogueTable` (`self.DialogueTableAsset`) _returnvalue)
  (`/Game/UI/WBP_DialogueBox.ShowLine` _returnvalue "Start")
  (`UserWidget.AddToViewport` _output_get 0)
  (add `/Game/UI/WBP_DialogueBox.OnDialogueClosed` _output_get (`|CreateDelegate` :!event `OnDialogueClosedHandler`)))

(event `/Game/Blueprints/Systems/BPI_Interactable.SetInteractionPromptVisible`
  (params (bVisible :type Boolean))
  (`SceneComponent.SetVisibility` (`self.InteractionWidget`) bVisible false))

(event `OnDialogueClosedHandler`
  (`Widget.RemoveFromParent` (`self.ActiveDialogueWidget`))
  (`/Game/Blueprints/Systems/BP_PlayerInteractionComponent.ExitDialogueMode` (`self.GetComponentByClass` (`self.OverlappingPlayer`) "/Game/Blueprints/Systems/BP_PlayerInteractionComponent.BP_PlayerInteractionComponent_C"))
  (message `/Game/Blueprints/Systems/BPI_Interactable.SetInteractionPromptVisible` self true))

(event `/Game/Blueprints/Systems/BPI_Interactable.ForceEndDialogue`
  (bind _activedialoguewidget (`self.ActiveDialogueWidget`))
  (`/Engine/EditorBlueprintResources/StandardMacros.IsValid` _activedialoguewidget
    (:`Is Valid`
      (`/Game/UI/WBP_DialogueBox.OnDialogueClosed` _activedialoguewidget))))

(fn `GetInteractionPrompt`
  (returns (PromptText :type Text))
  (return (`|FormatText` "(E) Talk to {Name}" (`self.NPCDisplayName`))))

(fn `UserConstructionScript`)